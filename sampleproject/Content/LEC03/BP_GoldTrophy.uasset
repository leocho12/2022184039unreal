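; BP_GoldTrophy is an actor that bobs up and down in place and explodes when its mesh is hit.
; It stores its spawn location on BeginPlay, then each Tick offsets Z by a time-based sine wave driven by Frequency and Amplitude.
; A component hit on the static mesh plays an explosion sound and particle effect at the actor's location, then destroys the actor.
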(event `self.ReceiveBeginPlay`
  (set `self.start_location` (`self.K2_GetActorLocation`)))

(event `self.ReceiveTick`
  (params (DeltaSeconds :type "Float (single-precision)"))
  (`self.K2_SetActorLocation` (+ (`self.start_location`) (`KismetMathLibrary.MakeVector` 0.0 0.0 (* (`KismetMathLibrary.Sin` (* (`GameplayStatics.GetTimeSeconds`) (`self.Frequency`) 6.283184)) (`self.Amplitude`))))))

(event `self.StaticMeshComponent.OnComponentHit`
  (params (HitComponent :type "PrimitiveComponent Object Reference") (OtherActor :type "Actor Object Reference") (OtherComp :type "PrimitiveComponent Object Reference") (NormalImpulse :type "Vector Structure") (Hit :type "HitResult Structure (by ref)"))
  (bind _returnvalue (`self.K2_GetActorLocation`))
  (`GameplayStatics.PlaySoundAtLocation` "/Game/StarterContent/Audio/Explosion_Cue.Explosion_Cue" _returnvalue (struct) 1.0 1.0 0.0 null null null null)
  (`GameplayStatics.SpawnEmitterAtLocation` "/Game/StarterContent/Particles/P_Explosion.P_Explosion" _returnvalue)
  (`self.K2_DestroyActor`))

(fn `UserConstructionScript`)